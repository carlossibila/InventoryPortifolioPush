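; Player inventory component that handles item pickup, money, health and their HUD widgets.
; A forward sphere trace each tick drives the interaction prompt; the interact input repeats it to add items to typed, fixed-size slot arrays, stacking up to DT_Item limits.
; Money grows on a delayed Tick, treating time as currency, and from BP_Money capsule overlaps valued through DT_Money.
; Health changes through debug keys and updates the health bar.
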(event Input|EnhancedActionEvents|EnhancedInputActionIA_Interact
  (params (ActionValue :type Boolean) (ElapsedSeconds :type Float%20%28double-precision%29) (TriggeredSeconds :type Float%20%28double-precision%29) (InputAction :type Input%20Action%20Object%20Reference :default "/Game/_GameMain/Inputs/IA_Interact.IA_Interact"))
  ;[0 0 0] pickup Item interaction
  (bind (_item _success _itemactor) (inventory|TraceItemtoPickUp))
  (if _success
    (bind _success_2 (inventory|AddtoInventory _item))
    (if _success_2
      (Actor|DestroyActor _itemactor)
      (Default|UpdateInventoryUI (Variables|widget|GetWBP_Inventory) (Variables|Default|GetInventoryArrays)))))

(event EventBeginPlay
  (bind _inventoryarrays (Variables|Default|GetInventoryArrays))
  (bind (_sword _shields _eatables) (Utilities|Struct|BreakS_ItemArray _inventoryarrays))
  ;[0 0 0] init
  (Utilities|FlowControl|Sequence
    (:then_0
      (Input|AddMappingContext (PlayerController|LocalPlayerSubsystems|GetEnhancedInputLocalPlayerSubsystem (Game|GetPlayerController 0)) "/Game/_GameMain/Inputs/IMC_Inventory.IMC_Inventory" 0 "(bIgnoreAllPressedKeysUntilRelease=True,bForceImmediately=False,bNotifyUserSettings=False)"))
    (:then_1
      (bind _returnvalue (UserInterface|CreateWidget "/Game/_GameMain/Widgets/WBP_Inventory.WBP_Inventory_C"))
      (Variables|widget|SetWBP_Inventory _returnvalue)
      (bind _asbp_third_person_character (Utilities|Casting|CastToBP_ThirdPersonCharacter (Game|GetPlayerCharacter 0)))
      (bind _output_get (Variables|Default|SetAs%20BP%20Third%20Person%20Character _asbp_third_person_character))
      (Collision|BindEventtoOnComponentBeginOverlap (Variables|/Script/Engine.Character|GetCapsuleComponent _output_get) (EventDispatchers|CreateEvent :!event PickUpMoney)))
    (:then_2
      (bind _returnvalue_2 (UserInterface|CreateWidget "/Game/_GameMain/Widgets/WBP_HealthBar.WBP_HealthBar_C"))
      (bind _output_get_2 (Variables|widget|SetWBP_HealthBar _returnvalue_2))
      (Class|UserWidget|SetPositioninViewport _output_get_2 "(X=30.000000,Y=30.000000)" true)
      (UserInterface|Viewport|AddtoViewport _output_get_2 0))
    (:then_3
      (bind _returnvalue_3 (UserInterface|CreateWidget "/Game/_GameMain/Widgets/WBP_Interaction.WBP_Interaction_C"))
      (Variables|widget|SetWBP_Interaction _returnvalue_3))
    (:then_4
      (Utilities|Array|Resize _sword 5)
      (Utilities|Array|Resize _shields 5)
      (Utilities|Array|Resize _eatables 10)
      (Default|UpdateInventoryUI (Variables|widget|GetWBP_Inventory) (Variables|Default|GetInventoryArrays)))
    (:then_5
      ;[1 0 0] REVIEW
      ;;[1 0 0.01969] moneyCount per time
      (bind _returnvalue_4 (UserInterface|CreateWidget "/Game/_GameMain/Widgets/WBP_MoneyTime.WBP_MoneyTime_C"))
      (bind _output_get_3 (Variables|widget|SetWBP_MoneyTime _returnvalue_4))
      (Class|UserWidget|SetPositioninViewport _output_get_3 "(X=720.000000,Y=30.000000)" true)
      (UserInterface|Viewport|AddtoViewport _output_get_3 0))))

(event EventTick
  (params (DeltaSeconds :type Float%20%28single-precision%29))
  (bind _wbp_interaction (Variables|widget|GetWBP_Interaction))
  (Utilities|FlowControl|Sequence
    (:then_0
      ;[1 0 0] REVIEW
      ;;[0.4072 0 0.01764] a ideia aqui é usar o tempo como currency, a conta do deltaSec muda o ammount, o delay muda o tempo com que essa funçao acontece
      (Utilities|FlowControl|Delay 1e+01)
      (bind _output_get (Variables|money|SetMoney_AmountFloat (+ (+ DeltaSeconds (* DeltaSeconds 1e+01)) (Variables|money|GetMoney_AmountFloat))))
      (Default|AmountFloattoTxt (Variables|widget|GetWBP_MoneyTime) _output_get))
    (:then_1
      ;[1 0 0.04338] event tick
      (bind (_item _success) (inventory|TraceItemtoPickUp))
      (Variables|/Game/_GameMain/Widgets/WBP_ItemInfo.WBP_ItemInfo_C|SetItem (Variables|/Game/_GameMain/Widgets/WBP_Interaction.WBP_Interaction_C|GetWBP_ItemInfo (Variables|widget|GetWBP_Interaction)) _item)
      (if _success
        (UserInterface|Viewport|AddtoViewport _wbp_interaction 0)
        (else
          (Widget|RemovefromParent _wbp_interaction))))))

(event Input|KeyboardEvents|N
  (params (Key :type Key%20Structure :default "None"))
  ;[0 0 0] debugLife
  (:Pressed
    (HealthBar|IncreaseHealth 0.5)))

(event Input|KeyboardEvents|M
  (params (Key :type Key%20Structure :default "None"))
  ;[0 0 0] debugLife
  (:Pressed
    (HealthBar|DecreaseHealth 0.5)))

(event Input|EnhancedActionEvents|EnhancedInputActionIA_ToggleInventory
  (params (ActionValue :type Boolean) (ElapsedSeconds :type Float%20%28double-precision%29) (TriggeredSeconds :type Float%20%28double-precision%29) (InputAction :type Input%20Action%20Object%20Reference :default "/Game/_GameMain/Inputs/IA_ToggleInventory.IA_ToggleInventory"))
  (bind _returnvalue (Game|GetPlayerController 0))
  (UserInterface|Viewport|AddtoViewport (Variables|widget|GetWBP_Inventory) 0)
  (Variables|/Script/Engine.PlayerController|SetbShowMouseCursor _returnvalue true)
  (Input|SetInputModeUIOnly _returnvalue (Variables|widget|GetWBP_Inventory) "DoNotLock" false))

(fn PickUpMoney
  (params (OverlappedComponent :type Primitive%20Component%20Object%20Reference) (OtherActor :type Actor%20Object%20Reference) (OtherComp :type Primitive%20Component%20Object%20Reference) (OtherBodyIndex :type Integer) (bFromSweep :type Boolean) (SweepResult :type Hit%20Result%20Structure%20%28by%20ref%29))
  (bind _asbp_money (Utilities|Casting|CastToBP_Money OtherActor))
  (bind _returnvalue (Utilities|GetDataTableRow "/Game/_GameMain/DataTables/DT_Money.DT_Money" (.rowname (Variables|/Game/_GameMain/Blueprints/BP_Money.BP_Money_C|GetMoney_DataTable _asbp_money)))
    (:then
      (bind _output_get (Variables|money|SetMoney_AmountFloat (+ (.value _returnvalue) (Variables|money|GetMoney_AmountFloat))))
      (Actor|DestroyActor _asbp_money)
      (Default|AmountFloattoTxt (Variables|widget|GetWBP_MoneyTime) _output_get)
      (return))))

(fn IncreaseHealth
  (params (healthToIncrease :type Float%20%28double-precision%29))
  (Variables|healthBar|SetHealth (+ healthToIncrease (Variables|healthBar|GetHealth)))
  (Default|UpdateHealthBar (Variables|widget|GetWBP_HealthBar)))

(fn DecreaseHealth
  (params (healthToDecrease :type Float%20%28double-precision%29))
  (Variables|healthBar|SetHealth (- (Variables|healthBar|GetHealth) healthToDecrease))
  (Default|UpdateHealthBar (Variables|widget|GetWBP_HealthBar)))

(fn TraceItemtoPickUp
  (bind _returnvalue (Game|GetPlayerCharacter 0))
  (bind _returnvalue_2 (Transformation|GetActorLocation _returnvalue))
  (bind _returnvalue_3 (- _returnvalue_2 "0.000000,0.000000,-1.000000"))
  (bind _outhit (Collision|SphereTraceByChannel _returnvalue_3 (+ _returnvalue_3 (* (Transformation|GetActorForwardVector _returnvalue) (Variables|Default|GetPickUpDistance))) 9e+01 "TraceTypeQuery1" false 0 "ForOneFrame"))
  (bind _asbp_item (Utilities|Casting|CastToBP_Item (.hitactor _outhit))
    (:then
      (return (Variables|/Game/_GameMain/Blueprints/BP_Item.BP_Item_C|GetItem _asbp_item) true (.hitactor _outhit)))
    (:CastFailed
      (return "" false 0))))

(fn AddtoInventory
  (params (Item :type S%20Slot%20Structure))
  (bind (_itemid _quantity _itemtype) (Utilities|Struct|BreakS_Slot Item))
  (bind (_itemid_2 _quantity_2 _itemtype_2) (Utilities|Struct|BreakS_Slot Item))
  (bind (_itemid_3 _quantity_3) (Utilities|Struct|BreakS_Slot Item))
  (bind (_itemid_4 _quantity_4) (Utilities|Struct|BreakS_Slot Item))
  (bind (_itemid_5 _quantity_5) (Utilities|Struct|BreakS_Slot Item))
  (bind (_itemid_6 _quantity_6 _itemtype_3) (Utilities|Struct|BreakS_Slot Item))
  (switch Utilities|FlowControl|Switch|SwitchonE_ItemType (.ItemType (Utilities|Struct|BreakS_Slot Item))
    (:NewEnumerator0
      ;[0 0 0] swords
      ;;[0 0 0] inventory item loop check
      (for (_array_element _array_index) (Utilities|Struct|BreakS_ItemArray (Variables|Default|GetInventoryArrays))
        ;;[0 0 0] add to item in inventory for swords
        (if (== (.RowName (Utilities|Struct|BreakDataTableRowHandle (.ItemID (Utilities|Struct|BreakS_Slot _array_element)))) (.RowName (Utilities|Struct|BreakDataTableRowHandle (.ItemID (Utilities|Struct|BreakS_Slot Item)))))
          (bind _returnvalue (Utilities|GetDataTableRow "/Game/_GameMain/DataTables/DT_Item.DT_Item" (.RowName (Utilities|Struct|BreakDataTableRowHandle _itemid_5)))
            (:then
              (if (>= (Utilities|Struct|BreakS_Item _returnvalue) (+ (.Quantity (Utilities|Struct|BreakS_Slot _array_element)) _quantity_5))
                (Utilities|Array|SetArrayElem (Utilities|Struct|BreakS_ItemArray (Variables|Default|GetInventoryArrays)) _array_index (Utilities|Struct|MakeS_Slot _itemid_6 (+ (.Quantity (Utilities|Struct|BreakS_Slot _array_element)) _quantity_5) _itemtype_3))
                (return true))))))
      ;;[0 0 0] create new slot for swords if none return from the add to item in inventory
      (for (_array_element_2 _array_index_2) (.Sword (Utilities|Struct|BreakS_ItemArray (Variables|Default|GetInventoryArrays)))
        (if (== (.Quantity (Utilities|Struct|BreakS_Slot _array_element_2)) 0)
          (Utilities|Array|SetArrayElem (.Sword (Utilities|Struct|BreakS_ItemArray (Variables|Default|GetInventoryArrays))) _array_index_2 Item)
          (return true)))
      (return false))
    (:NewEnumerator1
      ;[0 0 0] shields
      ;;[0 0 0] inventory item loop check
      (for (_array_element_3 _array_index_3) (Utilities|Struct|BreakS_ItemArray (Variables|Default|GetInventoryArrays))
        ;;[0 0 0] add to item in inventory for shields
        (if (== (.RowName (Utilities|Struct|BreakDataTableRowHandle (.ItemID (Utilities|Struct|BreakS_Slot _array_element_3)))) (.RowName (Utilities|Struct|BreakDataTableRowHandle (.ItemID (Utilities|Struct|BreakS_Slot Item)))))
          (bind _returnvalue_2 (Utilities|GetDataTableRow "/Game/_GameMain/DataTables/DT_Item.DT_Item" (.RowName (Utilities|Struct|BreakDataTableRowHandle _itemid_3)))
            (:then
              (if (>= (Utilities|Struct|BreakS_Item _returnvalue_2) (+ (.Quantity (Utilities|Struct|BreakS_Slot _array_element_3)) _quantity_3))
                (Utilities|Array|SetArrayElem (Utilities|Struct|BreakS_ItemArray (Variables|Default|GetInventoryArrays)) _array_index_3 (Utilities|Struct|MakeS_Slot _itemid_2 (+ (.Quantity (Utilities|Struct|BreakS_Slot _array_element_3)) _quantity_3) _itemtype_2))
                (return true))))))
      ;;[0 0 0] create new slot for shields if none return from the add to item in inventory
      (for (_array_element_4 _array_index_4) (Utilities|Struct|BreakS_ItemArray (Variables|Default|GetInventoryArrays))
        (if (== (.Quantity (Utilities|Struct|BreakS_Slot _array_element_4)) 0)
          (Utilities|Array|SetArrayElem (Utilities|Struct|BreakS_ItemArray (Variables|Default|GetInventoryArrays)) _array_index_4 Item)
          (return true)))
      (return false))
    (:NewEnumerator2
      ;[0 0 0] Eatables
      ;;[0 0 0] inventory item loop check
      (for (_array_element_5 _array_index_5) (.Eatables (Utilities|Struct|BreakS_ItemArray (Variables|Default|GetInventoryArrays)))
        ;;[0 0 0] add to item in inventory for eatables
        (if (== (Utilities|Struct|BreakDataTableRowHandle (.ItemID (Utilities|Struct|BreakS_Slot _array_element_5))) (.RowName (Utilities|Struct|BreakDataTableRowHandle (.ItemID (Utilities|Struct|BreakS_Slot Item)))))
          (bind _returnvalue_3 (Utilities|GetDataTableRow "/Game/_GameMain/DataTables/DT_Item.DT_Item" (.RowName (Utilities|Struct|BreakDataTableRowHandle _itemid_4)))
            (:then
              (if (>= (Utilities|Struct|BreakS_Item _returnvalue_3) (+ _quantity_4 (.Quantity (Utilities|Struct|BreakS_Slot _array_element_5))))
                (Utilities|Array|SetArrayElem (.Eatables (Utilities|Struct|BreakS_ItemArray (Variables|Default|GetInventoryArrays))) _array_index_5 (Utilities|Struct|MakeS_Slot _itemid (+ _quantity_4 (.Quantity (Utilities|Struct|BreakS_Slot _array_element_5))) _itemtype))
                (return true))))))
      ;;[0 0 0] create new slot for eatables if none return from the add to item in inventory
      (for (_array_element_6 _array_index_6) (.Eatables (Utilities|Struct|BreakS_ItemArray (Variables|Default|GetInventoryArrays)))
        (if (== (.Quantity (Utilities|Struct|BreakS_Slot _array_element_6)) 0)
          (Utilities|Array|SetArrayElem (.Eatables (Utilities|Struct|BreakS_ItemArray (Variables|Default|GetInventoryArrays))) _array_index_6 Item)
          (return true)))
      (return false))))